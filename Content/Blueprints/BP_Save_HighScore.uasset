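; BP_Save_HighScore holds the high score table as an array of score structs, capped at four entries.
; AddHighScore appends the new entry, calls SortSaveData, then trims the array.
; SortSaveData orders entries by descending score with a selection sort, repeatedly moving the result of DetermineHighestScoreValue into a temporary array.
; DetermineLowestScoreValue returns the weakest entry and its index, but nothing here calls it.
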(fn DetermineLowestScoreValue
  (for (_array_element _array_index) (Variables|Default|GetSaveStruct)
    (if (== _array_index 0)
      (LocalVariables|SetLowestScore_Local (.score _array_element))
      (LocalVariables|SetLowestIndex_local _array_index)
      (elif (< (.score _array_element) (LocalVariables|GetLowestScore_Local))
        (LocalVariables|SetLowestScore_Local (.score _array_element))
        (LocalVariables|SetLowestIndex_local _array_index))))
  (return (LocalVariables|GetLowestIndex_local) (Utilities|Array|Get(acopy) (Variables|Default|GetSaveStruct) (LocalVariables|GetLowestIndex_local))))

(fn DetermineHighestScoreValue
  (for (_array_element _array_index) (Variables|Default|GetSaveStruct)
    (if (== _array_index 0)
      (LocalVariables|SetHighestScore_Local (.score _array_element))
      (LocalVariables|SetHighestIndex_local _array_index)
      (elif (> (.score _array_element) (LocalVariables|GetHighestScore_Local))
        (LocalVariables|SetHighestScore_Local (.score _array_element))
        (LocalVariables|SetHighestIndex_local _array_index))))
  (return (LocalVariables|GetHighestIndex_local) (Utilities|Array|Get(acopy) (Variables|Default|GetSaveStruct) (LocalVariables|GetHighestIndex_local))))

(fn SortSaveData
  (while (> (Utilities|Array|Length (Variables|Default|GetSaveStruct)) 0)
    (bind (_highestscoreindex _highestscorestruct) (CallFunction|DetermineHighestScoreValue))
    (Utilities|Array|Add (LocalVariables|GetTempSaveStruct_Local) _highestscorestruct)
    (Utilities|Array|RemoveIndex (Variables|Default|GetSaveStruct) _highestscoreindex))
  (Variables|Default|SetSaveStruct (LocalVariables|GetTempSaveStruct_Local)))

(fn AddHighScore
  (params (NewScore :type STRUCT%20High%20Score%20Structure))
  (bind _savestruct (Variables|Default|GetSaveStruct))
  (Utilities|Array|Add (Variables|Default|GetSaveStruct) NewScore)
  (CallFunction|SortSaveData)
  (Utilities|Array|Resize _savestruct (Math|Integer|Min(Integer) 4 (Utilities|Array|Length _savestruct))))