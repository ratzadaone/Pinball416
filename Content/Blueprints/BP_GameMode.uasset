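; Pinball game mode that runs the game loop: main menu, ball lives, multiplied scoring and high-score qualification.
; Balls spawn at BP_Plunger, and each one's OnDestroyed event spawns the next or ends the game when none remain.
; Endgame opens high-score entry if the save is empty or Score reaches its lowest, otherwise the main menu.
; Reset restores class defaults; save data is lazily loaded or created, then cached.
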(event Custom|SpawnBall
  ;[1 1 1] Spawn / respawn Ball
  (bind _outactors (Actor|GetAllActorsOfClass "/Game/Blueprints/BP_Plunger.BP_Plunger_C"))
  (bind _returnvalue (Game|SpawnActorfromClass "/Game/Blueprints/BP_Ball.BP_Ball_C" (Math|Transform|MakeTransform (Default|GetBallSpawnLocation (Utilities|Array|Get(acopy) _outactors)) "0, 0, 0" "1,1,1") "Undefined" 0 0))
  (Game|BindEventtoOnDestroyed _returnvalue (delegate Custom|BallDestroyed)))

(event Custom|CreateHighScoreList
  ;[1 1 1] Create HighScoreList
  (bind _asbp_player_controller (Utilities|Casting|CastToBP_PlayerController (Game|GetPlayerController 0)))
  (bind _returnvalue (UserInterface|CreateWidget "/Game/Blueprints/HUD_HighScoreEntry.HUD_HighScoreEntry_C" _asbp_player_controller))
  (UserInterface|Viewport|AddtoViewport _returnvalue 0)
  (Variables|/Script/Engine.PlayerController|SetbShowMouseCursor _asbp_player_controller true)
  (Input|SetInputModeUIOnly _asbp_player_controller _returnvalue "LockAlways"))

(event Custom|BallDestroyed
  (params (DestroyedActor :type Actor%20Object%20Reference))
  ;[1 1 1] Spawn / respawn Ball
  (if (> (Variables|Default|GetBallsRemaining) 0)
    (CallFunction|SpawnBall)
    (bind _result (Math|Integer|DecrementInt (Variables|Default|GetBallsRemaining))
      (:%20%20
        (Development|PrintString (Utilities|String|ToString(Integer) _result))))
    (else
      (CallFunction|Endgame))))

(event Custom|CreateMainMenu
  ;[1 1 1] CreateMainMenu
  (CallFunction|GetSaveGameData)
  (Viewport|RemoveAllWidgets)
  (bind _asbp_player_controller (Utilities|Casting|CastToBP_PlayerController (Game|GetPlayerController 0)))
  (bind _returnvalue (UserInterface|CreateWidget "/Game/Blueprints/HUD_MainMenu.HUD_MainMenu_C" _asbp_player_controller))
  (UserInterface|Viewport|AddtoViewport _returnvalue 0)
  (Variables|/Script/Engine.PlayerController|SetbShowMouseCursor _asbp_player_controller true)
  (Input|SetInputModeUIOnly _asbp_player_controller _returnvalue "LockAlways"))

(event Custom|ResetGame
  (bind (_score _multiplier _ballsremaining) (Utilities|GetClassDefaults "BP_GameMode_C"))
  ;[1 1 1] Reset Game
  (Variables|Default|SetScore _score)
  (Variables|Default|SetMultiplier _multiplier)
  (Variables|Default|SetBallsRemaining _ballsremaining)
  (CallFunction|SpawnBall)
  (bind _asbp_player_controller (Utilities|Casting|CastToBP_PlayerController (Game|GetPlayerController 0)))
  (Default|CreatePlayerHUD _asbp_player_controller)
  (Variables|/Script/Engine.PlayerController|SetbShowMouseCursor _asbp_player_controller false)
  (Input|SetInputModeGameOnly _asbp_player_controller))

(event Custom|Endgame
  ;[1 1 1] Endgame
  (bind _currentsaveobj (CallFunction|GetSaveGameData))
  (if (<= (Utilities|Array|Length (Variables|/Game/Blueprints/BP_Save_HighScore.BP_Save_HighScore_C|GetSaveStruct _currentsaveobj)) 0)
    (CallFunction|CreateHighScoreList :!label _label)
    (else
      (bind _lowestscorestruct (Default|DetermineLowestScoreValue _currentsaveobj))
      (if (<= (.score _lowestscorestruct) (Variables|Default|GetScore))
        (goto _label)
        (else
          (CallFunction|CreateMainMenu))))))

(event EventBeginPlay
  ;[1 1 1] begin Play
  (CallFunction|CreateMainMenu))

(event EventTick
  (params (DeltaSeconds :type Float%20%28single-precision%29)))

(fn ConstructionScript)

(fn AddScore
  (params (PointsToAdd :type Float%20%28single-precision%29))
  ;[1 1 1] Add Score
  (bind _output_get (Variables|Default|SetScore (+ (* PointsToAdd (Variables|Default|GetMultiplier)) (Variables|Default|GetScore))))
  (return _output_get))

(fn GetSaveGameData
  (bind _currentsaveobj (Variables|Default|GetCurrentSaveObj)
    (:then
      (return _currentsaveobj))
    (:else
      (bind _returnvalue (SaveGame|DoesSaveGameExist (Variables|Default|GetHighScoreSaveName)))
      (if _returnvalue
        (bind _returnvalue_2 (SaveGame|LoadGamefromSlot (Variables|Default|GetHighScoreSaveName)))
        (bind _asbp_save_high_score (Utilities|Casting|CastToBP_Save_HighScore _returnvalue_2)
          (:then
            (Default|SortSaveData _asbp_save_high_score)
            (bind _output_get (Variables|Default|SetCurrentSaveObj _asbp_save_high_score))
            (return _output_get))
          (:CastFailed
            (return 0)))
        (else
          (bind _returnvalue_3 (SaveGame|CreateSaveGameObject "/Game/Blueprints/BP_Save_HighScore.BP_Save_HighScore_C"))
          (bind _output_get_2 (Variables|Default|SetCurrentSaveObj _returnvalue_3))
          (return _output_get_2))))))