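; BP_DropTargetSet is a bank of lettered drop targets that spells a word and raises the game mode's Multiplier when completed.
; The Construction Script uppercases DropTargetString and spawns one BP_DropTarget child actor per character, evenly spaced between Post1 and Post2, binding each OnDrop.
; ProcessDropTargets counts down TargetCounter and increments Multiplier at zero.
; The game mode's OnGameReset restores the counter to the string length.
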(event Custom|ProcessDropTargets
  (bind _result (Math|Integer|DecrementInt (Variables|Default|GetTargetCounter))
    (:%20%20
      (if (== _result 0)
        (bind _asbp_game_mode (Utilities|Casting|CastToBP_GameMode (Game|GetGameMode)))
        (Math|Float|IncrementFloat (Variables|/Game/Blueprints/BP_GameMode.BP_GameMode_C|GetMultiplier _asbp_game_mode))))))

(event Custom|ResetDroptargetCounter
  (Variables|Default|SetTargetCounter (Utilities|String|Len (Variables|Default|GetDropTargetString))))

(event EventBeginPlay
  (bind _asbp_game_mode (Utilities|Casting|CastToBP_GameMode (Game|GetGameMode)))
  (EventDispatchers|BindEventtoOnGameReset _asbp_game_mode (delegate Custom|ResetDroptargetCounter)))

(fn ConstructionScript
  (bind _post1 (Variables|Default|GetPost1))
  (|CallParentFunction)
  (bind _output_get (Variables|Default|SetDropTargetString (Class|KismetStringLibrary|ToUpper (Variables|Default|GetDropTargetString))))
  (for (_array_element _array_index) (Utilities|String|GetCharacterArrayfromString _output_get)
    (bind _returnvalue (AddComponent|AddChildActorComponent false (Math|Transform|MakeTransform (+ (* (Math|Vector|GetForwardVector _post1) (* (+ _array_index 1) (/ (Math|Vector|VectorLength (- (Variables|/Script/Engine.SceneComponent|GetRelativeLocation (Variables|Default|GetPost1)) (Variables|/Script/Engine.SceneComponent|GetRelativeLocation (Variables|Default|GetPost2)))) (Math|Conversions|ToFloat(Integer) (+ (Utilities|Array|Length (Utilities|String|GetCharacterArrayfromString _output_get)) 1))))) (* (Math|Vector|GetRightVector _post1) 2e+01)) (Variables|/Script/Engine.SceneComponent|GetRelativeRotation _post1) "1,1,1")))
    (bind _asbp_drop_target (Utilities|Casting|CastToBP_DropTarget (Variables|/Script/Engine.ChildActorComponent|GetChildActor _returnvalue)))
    (bind _output_get_2 (Variables|/Game/Blueprints/BP_DropTarget.BP_DropTarget_C|SetDropLetter _asbp_drop_target _array_element))
    (Rendering|Components|TextRender|SetText (Variables|/Game/Blueprints/BP_DropTarget.BP_DropTarget_C|GetDropText _asbp_drop_target) (Utilities|Text|ToText(String) _output_get_2))
    (EventDispatchers|BindEventtoOnDrop _asbp_drop_target (EventDispatchers|CreateEvent :!event Custom|ProcessDropTargets))))